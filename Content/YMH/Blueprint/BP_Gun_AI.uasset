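; BP_Gun_AI is a gun Blueprint that handles the aim-down-sights transition by moving its owner's spring arm.
; AimStartAction plays a timeline that lerps the spring arm's relative location from zero toward the GunMesh "Sight" socket, converted to gun-local space minus the AimOffset location.
; AimStopAction reverses the same timeline to ease back out.
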(event EventBeginPlay)

(event Collision|EventActorBeginOverlap
  (params (OtherActor :type Actor%20Object%20Reference)))

(event EventTick
  (params (DeltaSeconds :type Float%20%28single-precision%29)))

(event EventAimStartAction
  (bind _newtrack_0 (Timeline|Timeline Play)
    (:Update
      (Transformation|SetRelativeLocation (Actor|GetComponentbyClass (Components|GetOwner) "/Script/Engine.SpringArmComponent") (Math|Vector|Lerp(Vector) "0, 0, 0" (- (Math|Transform|InverseTransformLocation (Transformation|GetActorTransform) (Transformation|GetSocketLocation (Variables|Default|GetGunMesh) "Sight")) (Variables|/Script/Engine.SceneComponent|GetRelativeLocation (Variables|Default|GetAimOffset))) _newtrack_0) false false))))

(event EventAimStopAction
  (bind _newtrack_0 (Timeline|Timeline Reverse)
    (:Update
      (Transformation|SetRelativeLocation (Actor|GetComponentbyClass (Components|GetOwner) "/Script/Engine.SpringArmComponent") (Math|Vector|Lerp(Vector) "0, 0, 0" (- (Math|Transform|InverseTransformLocation (Transformation|GetActorTransform) (Transformation|GetSocketLocation (Variables|Default|GetGunMesh) "Sight")) (Variables|/Script/Engine.SceneComponent|GetRelativeLocation (Variables|Default|GetAimOffset))) _newtrack_0) false false))))

(fn ConstructionScript)