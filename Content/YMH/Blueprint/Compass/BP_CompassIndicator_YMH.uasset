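; Component that registers its owning actor on the player's compass HUD as an icon.
; Shortly after BeginPlay it creates a compass icon widget for the owner and adds it to the player's compass overlay.
; Wayout indicators always get an icon; others need their objective component's ID to match one in the player's quest log.
; The nested loop breaks limit that search to the first stage of the first quest.
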(event EventBeginPlay
  (bind _returnvalue (Components|GetOwner))
  (bind _returnvalue_2 (Actor|GetComponentbyClass _returnvalue "/Game/YMH/Blueprint/QuestSystem/BP_ObjectiveComp_YMH.BP_ObjectiveComp_YMH_C"))
  (Utilities|FlowControl|Delay 0.2)
  (bind _asbp_character_osh (Utilities|Casting|CastToBP_Character_OSH (Game|GetPlayerCharacter 0)))
  (Utilities|IsValid _asbp_character_osh
    (:Is%20Valid
      (if (Variables|Default|GetbWayout)
        (bind _returnvalue_3 (UserInterface|CreateWidget "/Game/YMH/Blueprint/Compass/WBP_CompassIcon_YMH.WBP_CompassIcon_YMH_C" 0 (Variables|Default|GetIcon) (Components|GetOwner) :!label _label))
        (Widget|Panel|AddChild (Variables|/Game/YMH/Blueprint/Compass/WBP_Compass_YMH.WBP_Compass_YMH_C|GetCompassOverlay (Variables|/Game/YMH/Blueprint/Compass/WBP_CompassHUD_YMH.WBP_CompassHUD_YMH_C|GetWBP_Compass_YMH (Variables|/Game/YMH/Blueprint/Compass/BP_CompassComp_YMH.BP_CompassComp_YMH_C|GetCompassHUD (Variables|/Game/OSH/Blueprint/Character/BP_Character_OSH.BP_Character_OSH_C|GetBP_CompassComp_YMH _asbp_character_osh)))) _returnvalue_3)
        (else
          (Utilities|IsValid _returnvalue_2
            (:Is%20Valid
              (Variables|Default|SetHasQuest false)
              (bind _array_element (Utilities|Array|ForEachLoopwithBreak (Variables|/Script/SesacProject5.QuestLogComponent|GetquestList (Actor|GetComponentbyClass _asbp_character_osh "/Game/YMH/Blueprint/QuestSystem/BP_QuestLogComponent_YMH.BP_QuestLogComponent_YMH_C")) :!label _label_2)
                (:LoopBody
                  (bind _array_element_2 (Utilities|Array|ForEachLoopwithBreak (Utilities|Struct|BreakQuestDetails (Utilities|Struct|BreakQuestManagement _array_element)) :!label _label_3)
                    (:LoopBody
                      (bind _array_element_3 (Utilities|Array|ForEachLoopwithBreak (Utilities|Struct|BreakStageDetails _array_element_2) :!label _label_4)
                        (:LoopBody
                          (if (Utilities|Enum|Equal(Enum) (Variables|/Script/SesacProject5.ObjectiveComponent|GetobjectID _returnvalue_2) (Utilities|Struct|BreakObjectiveDetails _array_element_3))
                            (Variables|Default|SetHasQuest true)
                            (goto _label_4 Break)))
                        (:Completed
                          (goto _label_3 Break))))
                    (:Completed
                      (goto _label_2 Break))))
                (:Completed
                  (if (Variables|Default|GetHasQuest)
                    (goto _label)))))))))))