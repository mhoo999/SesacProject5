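; BP_CompassComp_YMH is an actor component that sets up the compass HUD for the local player's character.
; On BeginPlay, if the owning Character is controlled by player controller 0, it creates WBP_CompassHUD_YMH and adds it to the viewport.
; It then takes the exit array from the character's EscapeComponent and assigns the flag icon to each exit's BP_CompassIndicator_YMH.
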(event EventBeginPlay
  (bind _ascharacter (Utilities|Casting|CastToCharacter (Components|GetOwner)))
  (if (== (Game|GetPlayerController 0) (Pawn|GetController _ascharacter))
    (bind _returnvalue (UserInterface|CreateWidget "/Game/YMH/Blueprint/Compass/WBP_CompassHUD_YMH.WBP_CompassHUD_YMH_C"))
    (bind _output_get (Variables|Default|SetCompassHUD _returnvalue))
    (UserInterface|Viewport|AddtoViewport _output_get 0)
    (for _array_element (Class|EscapeComponent|GetExitArray (Actor|GetComponentbyClass _ascharacter "/Script/SesacProject5.EscapeComponent"))
      (Variables|/Game/YMH/Blueprint/Compass/BP_CompassIndicator_YMH.BP_CompassIndicator_YMH_C|SetIcon (Actor|GetComponentbyClass _array_element "/Game/YMH/Blueprint/Compass/BP_CompassIndicator_YMH.BP_CompassIndicator_YMH_C") "/Game/Resource/YMH/CompassIcon/CompassIcon_Flag.CompassIcon_Flag"))))

(event EventTick
  (params (DeltaSeconds :type Float%20%28single-precision%29)))