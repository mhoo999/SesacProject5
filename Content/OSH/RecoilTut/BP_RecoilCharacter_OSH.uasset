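; BP_RecoilCharacter_OSH is a player character that carries an AK weapon and can aim down its sight.
; On BeginPlay it snaps the camera to a mesh socket, then spawns the weapon and attaches it to the right-hand socket.
; Holding right mouse sets IsAim and has the weapon attach the camera to its sight; releasing returns it to the mesh.
; Axis inputs drive movement and look, and a debug C key toggles crouch.
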(event EventBeginPlay
  (Transformation|AttachComponentToComponent (Variables|Default|GetCamera) (Variables|Character|GetMesh) "Camera" "SnapToTarget" "KeepWorld" "KeepWorld" true)
  (bind _returnvalue (Game|SpawnActorfromClass "/Game/OSH/RecoilTut/BP_Weapon_AK_OSH.BP_Weapon_AK_OSH_C" (Math|Transform|MakeTransform "0, 0, 0" "0, 0, 0" "1.000000,1.000000,1.000000") "AlwaysSpawn" "MultiplyWithRoot" 0 0))
  (bind _output_get (Variables|Default|SetWeapon _returnvalue))
  (Transformation|AttachComponentToComponent _output_get (Variables|Character|GetMesh) "Weapon_R" "SnapToTarget" "SnapToTarget" "SnapToTarget" true))

(event Collision|EventActorBeginOverlap
  (params (OtherActor :type Actor%20Object%20Reference)))

(event Input|AxisEvents|InputAxisMoveForward/Backward
  (params (AxisValue :type Float%20%28single-precision%29))
  (Pawn|Input|AddMovementInput (Transformation|GetActorForwardVector) AxisValue false))

(event Input|AxisEvents|InputAxisLookUp/DownMouse
  (params (AxisValue :type Float%20%28single-precision%29))
  (Pawn|Input|AddControllerPitchInput AxisValue))

(event Input|AxisEvents|InputAxisMoveRight/Left
  (params (AxisValue :type Float%20%28single-precision%29))
  (Pawn|Input|AddMovementInput (Transformation|GetActorRightVector) AxisValue false))

(event Input|AxisEvents|InputAxisTurnRight/LeftMouse
  (params (AxisValue :type Float%20%28single-precision%29))
  (Pawn|Input|AddControllerYawInput AxisValue))

(event Input|MouseEvents|DebugKeyRightMouseButton
  (params (Key :type Key%20Structure :default "None") (ActionValue :type Input%20Action%20Value%20Structure))
  (:Pressed
    (Variables|Default|SetbIsAim true)
    (Default|AttachtoSight (Variables|Default|GetWeapon) (Variables|Default|GetCamera)))
  (:Released
    (Variables|Default|SetbIsAim false)
    (Transformation|AttachComponentToComponent (Variables|Default|GetCamera) (Variables|Character|GetMesh) "Camera" "SnapToTarget" "KeepWorld" "KeepWorld" true)))

(event Input|KeyboardEvents|DebugKeyC
  (params (Key :type Key%20Structure :default "None") (ActionValue :type Input%20Action%20Value%20Structure))
  (:Pressed
    (if (Variables|Default|GetbIsCrouched)
      (Character|UnCrouch)
      (else
        (Character|Crouch)))))

(fn ConstructionScript)