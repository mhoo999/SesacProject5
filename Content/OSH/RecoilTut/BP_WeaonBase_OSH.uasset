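; Base weapon Blueprint that handles socket-based attachment, a fire mode toggle and empty start and stop fire events.
; It attaches to its owning Character's mesh at a weapon socket and flips between Single and Automatic fire.
; It can snap a given camera to the sight socket while keeping world rotation, and exposes world-space muzzle and sight transforms from the skeletal mesh.
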(event Custom|AttachToCharacter
  (bind _ascharacter (Utilities|Casting|CastToCharacter (Components|GetOwner)))
  (bind _output_get (Variables|Default|SetCharacter _ascharacter))
  (Transformation|AttachComponentToComponent (Variables|/Script/Engine.Character|GetMesh _output_get) (Variables|Default|GetWeaponSocketName) "SnapToTarget" "SnapToTarget" "SnapToTarget" true))

(event Custom|Attach%20To%20Sight
  (params (Camera :type Camera%20Component%20Object%20Reference))
  (Transformation|AttachComponentToComponent Camera (Variables|Default|GetSkeletalMesh) (Variables|Default|GetSightSocketName) "SnapToTarget" "KeepWorld" "KeepWorld" true)
  (Transformation|SetRelativeLocation Camera "0, 0, 0" false false))

(event Custom|ToggleFireMode
  (switch Utilities|FlowControl|Switch|SwitchonEFireMode (Variables|Default|GetFireMode)
    (:NewEnumerator1
      (Variables|Default|SetFireMode "NewEnumerator2"))
    (:NewEnumerator2
      (Variables|Default|SetFireMode "NewEnumerator1"))))

(event Custom|CE_StopFire)

(event Custom|CE_OnFire)

(event EventBeginPlay)

(event Collision|EventActorBeginOverlap
  (params (OtherActor :type Actor%20Object%20Reference)))

(event EventTick
  (params (DeltaSeconds :type Float%20%28single-precision%29)))

(fn ConstructionScript)

(fn GetMuzzleTransform
  (return (Transformation|GetSocketTransform (Variables|Default|GetSkeletalMesh) (Variables|Default|GetMuzzleSocketName) "RTS_World")))

(fn GetSightTransform
  (return (Transformation|GetSocketTransform (Variables|Default|GetSkeletalMesh) (Variables|Default|GetSightSocketName) "RTS_World")))