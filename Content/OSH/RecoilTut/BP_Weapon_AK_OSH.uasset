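; AK weapon Blueprint that applies camera recoil while firing and recovers aim afterwards.
; Firing plays RecoilTimeline, feeding its pitch and yaw curves into player controller input.
; Stopping reverses the timeline at higher speed with negated, amplified input, multiplied by a range-mapped factor from the pitch offset between stored origin and post-recoil rotations.
; DoOnce gates capture both rotations and reset when the reverse finishes.
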(event Custom|CE_ResetRecoil
  (Utilities|FlowControl|Sequence
    (:then_0
      (Utilities|FlowControl|DoOnce false) ; enters at Reset
    )
    (:then_1
      (Utilities|FlowControl|DoOnce false) ; enters at Reset
    )))

(event EventBeginPlay)

(event Collision|EventActorBeginOverlap
  (params (OtherActor :type Actor%20Object%20Reference)))

(event EventTick
  (params (DeltaSeconds :type Float%20%28single-precision%29)))

(event EventCEonFire
  (bind _returnvalue (Game|GetPlayerController 0))
  (bind _returnvalue_2 (Pawn|GetControlRotation _returnvalue :!class /Script/Engine.Controller))
  (Components|Timeline|SetPlayRate (Variables|Default|GetRecoilTimeline) 1.0)
  (Utilities|FlowControl|Sequence
    (:then_0
      (Utilities|FlowControl|DoOnce false
        (:Completed
          (Variables|Default|SetOriginRotation _returnvalue_2))))
    (:then_1
      (bind (_direction _pitchinput _yawinput) (Timeline|RecoilTimeline Play)
        (:Update
          (Development|PrintString (Utilities|String|ToString(Float) (.Pitch (Math|Rotator|BreakRotator (Math|Rotator|Delta(Rotator) (Variables|Default|GetOriginRotation) _returnvalue_2)))))
          (switch Utilities|FlowControl|Switch|SwitchonETimelineDirection _direction
            (:Forward
              (CallFunction|UpdatePlayerPitchandYawInput _pitchinput _yawinput))
            (:Backward
              (Utilities|FlowControl|Sequence
                (:then_0
                  (Utilities|FlowControl|DoOnce false
                    (:Completed
                      (Variables|Default|SetPostRecoilRotation (Pawn|GetControlRotation (Game|GetPlayerController 0) :!class /Script/Engine.Controller)))))
                (:then_1
                  (CallFunction|UpdatePlayerPitchandYawInput (* _pitchinput -13.0 (Math|Float|SelectFloat (Math|Float|MapRangeClamped (Math|Float|Absolute(Float) (.Pitch (Math|Rotator|BreakRotator (Math|Rotator|Delta(Rotator) (Variables|Default|GetOriginRotation) (Variables|Default|GetPostRecoilRotation))))) 0.0 (Variables|Default|GetRecoilMaxThreashold) 0.0 1.0) (Math|Float|MapRangeClamped (Math|Float|Absolute(Float) (.Pitch (Math|Rotator|BreakRotator (Math|Rotator|Delta(Rotator) (Variables|Default|GetOriginRotation) (Variables|Default|GetPostRecoilRotation))))) (Variables|Default|GetRecoilMaxThreashold) 3e+01 1.0 0.0) (> (Math|Float|Absolute(Float) (.Pitch (Math|Rotator|BreakRotator (Math|Rotator|Delta(Rotator) (Variables|Default|GetOriginRotation) (Variables|Default|GetPostRecoilRotation))))) (Variables|Default|GetRecoilMaxThreashold)))) (* _yawinput -3.0 (Math|Float|SelectFloat (Math|Float|MapRangeClamped (Math|Float|Absolute(Float) (.Pitch (Math|Rotator|BreakRotator (Math|Rotator|Delta(Rotator) (Variables|Default|GetOriginRotation) (Variables|Default|GetPostRecoilRotation))))) 0.0 (Variables|Default|GetRecoilMaxThreashold) 0.0 1.0) (Math|Float|MapRangeClamped (Math|Float|Absolute(Float) (.Pitch (Math|Rotator|BreakRotator (Math|Rotator|Delta(Rotator) (Variables|Default|GetOriginRotation) (Variables|Default|GetPostRecoilRotation))))) (Variables|Default|GetRecoilMaxThreashold) 3e+01 1.0 0.0) (> (Math|Float|Absolute(Float) (.Pitch (Math|Rotator|BreakRotator (Math|Rotator|Delta(Rotator) (Variables|Default|GetOriginRotation) (Variables|Default|GetPostRecoilRotation))))) (Variables|Default|GetRecoilMaxThreashold))))))))))
        (:Finished
          (switch Utilities|FlowControl|Switch|SwitchonETimelineDirection _direction
            (:Backward
              (CallFunction|CEResetRecoil))))))))

(event EventCEStopFire
  (Components|Timeline|SetPlayRate (Variables|Default|GetRecoilTimeline) 13.0)
  (bind (_direction _pitchinput _yawinput) (Timeline|RecoilTimeline Reverse)
    (:Update
      (Development|PrintString (Utilities|String|ToString(Float) (.Pitch (Math|Rotator|BreakRotator (Math|Rotator|Delta(Rotator) (Variables|Default|GetOriginRotation) (Pawn|GetControlRotation (Game|GetPlayerController 0) :!class /Script/Engine.Controller))))))
      (switch Utilities|FlowControl|Switch|SwitchonETimelineDirection _direction
        (:Forward
          (CallFunction|UpdatePlayerPitchandYawInput _pitchinput _yawinput))
        (:Backward
          (Utilities|FlowControl|Sequence
            (:then_0
              (Utilities|FlowControl|DoOnce false
                (:Completed
                  (Variables|Default|SetPostRecoilRotation (Pawn|GetControlRotation (Game|GetPlayerController 0) :!class /Script/Engine.Controller)))))
            (:then_1
              (CallFunction|UpdatePlayerPitchandYawInput (* _pitchinput -13.0 (Math|Float|SelectFloat (Math|Float|MapRangeClamped (Math|Float|Absolute(Float) (.Pitch (Math|Rotator|BreakRotator (Math|Rotator|Delta(Rotator) (Variables|Default|GetOriginRotation) (Variables|Default|GetPostRecoilRotation))))) 0.0 (Variables|Default|GetRecoilMaxThreashold) 0.0 1.0) (Math|Float|MapRangeClamped (Math|Float|Absolute(Float) (.Pitch (Math|Rotator|BreakRotator (Math|Rotator|Delta(Rotator) (Variables|Default|GetOriginRotation) (Variables|Default|GetPostRecoilRotation))))) (Variables|Default|GetRecoilMaxThreashold) 3e+01 1.0 0.0) (> (Math|Float|Absolute(Float) (.Pitch (Math|Rotator|BreakRotator (Math|Rotator|Delta(Rotator) (Variables|Default|GetOriginRotation) (Variables|Default|GetPostRecoilRotation))))) (Variables|Default|GetRecoilMaxThreashold)))) (* _yawinput -3.0 (Math|Float|SelectFloat (Math|Float|MapRangeClamped (Math|Float|Absolute(Float) (.Pitch (Math|Rotator|BreakRotator (Math|Rotator|Delta(Rotator) (Variables|Default|GetOriginRotation) (Variables|Default|GetPostRecoilRotation))))) 0.0 (Variables|Default|GetRecoilMaxThreashold) 0.0 1.0) (Math|Float|MapRangeClamped (Math|Float|Absolute(Float) (.Pitch (Math|Rotator|BreakRotator (Math|Rotator|Delta(Rotator) (Variables|Default|GetOriginRotation) (Variables|Default|GetPostRecoilRotation))))) (Variables|Default|GetRecoilMaxThreashold) 3e+01 1.0 0.0) (> (Math|Float|Absolute(Float) (.Pitch (Math|Rotator|BreakRotator (Math|Rotator|Delta(Rotator) (Variables|Default|GetOriginRotation) (Variables|Default|GetPostRecoilRotation))))) (Variables|Default|GetRecoilMaxThreashold))))))))))
    (:Finished
      (switch Utilities|FlowControl|Switch|SwitchonETimelineDirection _direction
        (:Backward
          (CallFunction|CEResetRecoil))))))

(fn ConstructionScript
  (|CallParentFunction))

(fn UpdatePlayerPitchandYawInput
  (params (Val :type Float%20%28single-precision%29) (Val2 :type Float%20%28single-precision%29))
  (bind _returnvalue (Game|GetPlayerController 0))
  (Class|PlayerController|AddPitchInput _returnvalue Val)
  (Class|PlayerController|AddYawInput _returnvalue Val2))