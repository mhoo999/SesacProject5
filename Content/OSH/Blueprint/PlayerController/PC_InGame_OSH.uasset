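; In-game player controller that handles the ToggleTabWidget event for the compass HUD and the tab menu's quest display.
; The event finds the compass component on the controlled pawn and flips its HUD between Hidden and HitTestInvisible, checking validity only before showing it.
; After either visibility change it refreshes the quest widget through the InGameWidget's TabWidget, whose own visibility is not changed here.
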(event EventBeginPlay)

(event EventTick
  (params (DeltaSeconds :type Float%20%28single-precision%29)))

(event EventToggleTabWidget
  (bind _returnvalue (Pawn|GetControlledPawn))
  (bind _returnvalue_2 (Actor|GetComponentbyClass _returnvalue "/Game/YMH/Blueprint/Compass/BP_CompassComp_YMH.BP_CompassComp_YMH_C"))
  (bind _compasshud (Variables|/Game/YMH/Blueprint/Compass/BP_CompassComp_YMH.BP_CompassComp_YMH_C|GetCompassHUD _returnvalue_2))
  (if (Utilities|Enum|Equal(Enum) (Widget|GetVisibility (Variables|/Game/YMH/Blueprint/Compass/BP_CompassComp_YMH.BP_CompassComp_YMH_C|GetCompassHUD _returnvalue_2)) "HitTestInvisible")
    (Widget|SetVisibility _compasshud "Hidden")
    (else
      (Utilities|IsValid _compasshud
        (:Is%20Valid
          (Widget|SetVisibility _compasshud "HitTestInvisible")))))
  (Class|TabWidget|RefreshQuestWidget (Variables|/Script/SesacProject5.InGameWidget|GetTabWidget (Variables|Default|GetInGameWidget))))

(fn ConstructionScript)