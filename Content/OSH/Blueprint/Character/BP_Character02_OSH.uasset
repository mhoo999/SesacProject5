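; BP_Character02_OSH is an FPS character Blueprint that adds a crosshair and a networked rifle reload animation.
; After parent BeginPlay, it creates the crosshair widget only if controlled by player controller 0.
; A debug R key sends a server RPC that multicasts the reload montage, with no ammo logic.
; The multicast zeroes left-hand IK alpha on the anim instance, then restores it after a delay equal to the montage length.
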(event Custom|MultiRPC_PlayReloadMontage
  (bind _asabp_fps_poly_osh (Utilities|Casting|CastToABP_FPS_Poly_OSH (Components|SkeletalMesh|GetAnimInstance (Variables|Character|GetMesh))))
  (Class|FPSAnimInstance|SetLeftHandIKAlpha _asabp_fps_poly_osh 0.0)
  (bind _returnvalue (Animation|PlayAnimMontage "/Game/OSH/Animation/Montage/AM_Reload_Rifle_Ironsights.AM_Reload_Rifle_Ironsights" 1.0 "None"))
  (Utilities|FlowControl|Delay _returnvalue)
  (bind _asabp_fps_poly_osh_2 (Utilities|Casting|CastToABP_FPS_Poly_OSH (Components|SkeletalMesh|GetAnimInstance (Variables|Character|GetMesh))))
  (Class|FPSAnimInstance|SetLeftHandIKAlpha _asabp_fps_poly_osh_2 1.0))

(event Custom|ServerRPC_PlayReloadMontage
  (CallFunction|MultiRPCPlayReloadMontage))

(event EventBeginPlay
  (|CallParentFunction)
  (if (== (Pawn|GetController) (Game|GetPlayerController 0))
    (bind _returnvalue (UserInterface|CreateWidget "/Game/OSH/FPSTut/WBP_Crosshair.WBP_Crosshair_C"))
    (UserInterface|Viewport|AddtoViewport _returnvalue 0)))

(event Input|KeyboardEvents|DebugKeyR
  (params (Key :type Key%20Structure :default "None") (ActionValue :type Input%20Action%20Value%20Structure))
  (:Pressed
    (CallFunction|ServerRPCPlayReloadMontage)))

(fn ConstructionScript)